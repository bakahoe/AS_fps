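; BP_Target is a moving shooting target that takes a set number of hits before being destroyed.
; Each tick it offsets itself along a normalized Direction scaled by Speed per frame, without delta time, while a looping timer reverses Direction every MovementDuration.
; The Hit event decrements HitPoints and plays an explosion sound, adding a Niagara effect and destroying the actor when they run out.
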(event Custom|FlipDirection
  ;[0.15 0.03517 0.1437 0.5] flippy
  (Variables|Default|SetDirection (* (Variables|Default|GetDirection) -1.0)))

(event EventBeginPlay
  ;[0.15 0.03517 0.1437 0.5] flippy
  (Utilities|Time|SetTimerbyEvent (delegate Custom|FlipDirection) (Variables|Default|GetMovementDuration) true))

(event Collision|EventActorBeginOverlap
  (params (OtherActor :type Actor%20Object%20Reference)))

(event EventTick
  (params (DeltaSeconds :type Float%20%28single-precision%29))
  ;[0.001563 0.15 0.1392 0.5] target movement
  (Transformation|AddActorWorldOffset (* (Math|Vector|Normalize (Variables|Default|GetDirection)) (Variables|Default|GetSpeed))))

(event Collision|EventHit
  (params (MyComp :type Primitive%20Component%20Object%20Reference) (Other :type Actor%20Object%20Reference) (OtherComp :type Primitive%20Component%20Object%20Reference) (bSelfMoved :type Boolean) (HitLocation :type Vector :default "0, 0, 0") (HitNormal :type Vector :default "0, 0, 0") (NormalImpulse :type Vector :default "0, 0, 0") (Hit :type Hit%20Result%20Structure%20%28by%20ref%29))
  ;[0.15 0.05189 0.001273 0.5] Target hit
  (Variables|Default|SetHitPoints (- (Variables|Default|GetHitPoints) 1))
  (if (<= (Variables|Default|GetHitPoints) 0)
    ;[0.15 0.1486 0.007812 0.5] Destroy Target
    (Niagara|SpawnSystematLocation "/Game/0_fps/FX/PE_TargetHit.PE_TargetHit" HitLocation)
    (Audio|SpawnSoundatLocation "/Game/0_fps/Audio/MP3_Explosions_Small.MP3_Explosions_Small" HitLocation "0, 0, 0" 1.0 1.0 0.0 0 0)
    (Actor|DestroyActor)
    (else
      (Audio|PlaySoundatLocation "/Game/0_fps/Audio/MP3_Explosions_Small.MP3_Explosions_Small" HitLocation "0, 0, 0" 1.0 1.0 0.0 0 0 0 0))))

(fn ConstructionScript)