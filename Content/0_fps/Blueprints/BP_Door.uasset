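; A key-locked door with a status light that responds to the first-person player entering its collision volume.
; BeginPlay caches the player character and gives the light mesh a dynamic material instance.
; On overlap the light brightens, turning red without HasKey, or green with it while a reversed Timeline drives the door's rotation lerp.
; Leaving restores the default light and plays the Timeline forward, whether or not the player holds the key.
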(event OnComponentBeginOverlap(Collision)
  (params (OverlappedComponent :type Primitive%20Component%20Object%20Reference) (OtherActor :type Actor%20Object%20Reference) (OtherComp :type Primitive%20Component%20Object%20Reference) (OtherBodyIndex :type Integer) (bFromSweep :type Boolean) (SweepResult :type Hit%20Result%20Structure%20%28by%20ref%29))
  (bind _dynamicmaterial (Variables|Default|GetDynamicMaterial))
  ;[0.8906 0.2007 0.7844 0.5] Light Change
  (if (== OtherActor (Variables|Default|GetBP_FirstPersonCharacter))
    (Rendering|Material|SetScalarParameterValue _dynamicmaterial "Intensity" 1e+02 :!class /Script/Engine.MaterialInstanceDynamic)
    (if (Variables|/Game/0_fps/Blueprints/BP_FirstPersonCharacter.BP_FirstPersonCharacter_C|GetHasKey (Variables|Default|GetBP_FirstPersonCharacter))
      (Rendering|Material|SetVectorParameterValue _dynamicmaterial "Colour" "(R=0.015556,G=0.442708,B=0.120101,A=1.000000)" :!class /Script/Engine.MaterialInstanceDynamic)
      ;[0.01576 0.01305 0.15 0.5] door anim
      (bind _alpha (Timeline|Timeline Reverse)
        (:Update
          (Transformation|SetRelativeRotation (Variables|Default|GetSM_Door) (Math|Rotator|Lerp(Rotator) "0, 0, 0" "0.000000,90.000000,0.000000" _alpha) false false)))
      (else
        (Rendering|Material|SetVectorParameterValue _dynamicmaterial "Colour" "(R=0.765217,G=0.000000,B=0.078910,A=1.000000)" :!class /Script/Engine.MaterialInstanceDynamic)))))

(event OnComponentEndOverlap(Collision)
  (params (OverlappedComponent :type Primitive%20Component%20Object%20Reference) (OtherActor :type Actor%20Object%20Reference) (OtherComp :type Primitive%20Component%20Object%20Reference) (OtherBodyIndex :type Integer))
  (bind _dynamicmaterial (Variables|Default|GetDynamicMaterial))
  ;[0.5938 0.0402 0.0486 0.5] Return to default
  (if (== OtherActor (Variables|Default|GetBP_FirstPersonCharacter))
    (Rendering|Material|SetScalarParameterValue _dynamicmaterial "Intensity" 1.0 :!class /Script/Engine.MaterialInstanceDynamic)
    (Rendering|Material|SetVectorParameterValue _dynamicmaterial "Colour" "(R=1.000000,G=0.974870,B=0.437500,A=1.000000)" :!class /Script/Engine.MaterialInstanceDynamic)
    ;[0.01576 0.01305 0.15 0.5] door anim
    (bind _alpha (Timeline|Timeline Play)
      (:Update
        (Transformation|SetRelativeRotation (Variables|Default|GetSM_Door) (Math|Rotator|Lerp(Rotator) "0, 0, 0" "0.000000,90.000000,0.000000" _alpha) false false)))))

(event EventBeginPlay
  ;[0.01406 0.15 0.148 0.5] Setup
  (bind _asbp_first_person_character (Utilities|Casting|CastToBP_FirstPersonCharacter (Game|GetPlayerCharacter 0)))
  (Variables|Default|SetBP_FirstPersonCharacter _asbp_first_person_character)
  (bind _returnvalue (Rendering|Material|CreateDynamicMaterialInstance "/Game/0_fps/Materials/MI_DoorLight.MI_DoorLight" "None" "None" :!class /Script/Engine.KismetMaterialLibrary))
  (Variables|Default|SetDynamicMaterial _returnvalue)
  (Rendering|Material|SetMaterial (Variables|Default|GetSM_Light) 0 (Variables|Default|GetDynamicMaterial)))

(event EventTick
  (params (DeltaSeconds :type Float%20%28single-precision%29)))

(fn ConstructionScript)