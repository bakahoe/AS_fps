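; BP_Key is a key actor apparently meant to appear once the level's BP_Target actors are gone.
; Each Tick it adds an element to the fetched target array and prints the returned index.
; Visibility, collision and a one-time particle and sound effect depend on that index being below zero, a condition an Add index never meets.
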(event EventBeginPlay)

(event Collision|EventActorBeginOverlap
  (params (OtherActor :type Actor%20Object%20Reference)))

(event EventTick
  (params (DeltaSeconds :type Float%20%28single-precision%29))
  (bind _defaultsceneroot (Variables|Default|GetDefaultSceneRoot))
  (bind _returnvalue (Transformation|GetWorldLocation _defaultsceneroot))
  ;[0.9062 0.151 0.8236 0.5] Key Visi
  (bind _outactors (Actor|GetAllActorsOfClass "/Game/0_fps/Blueprints/BP_Target.BP_Target_C"))
  (bind _returnvalue_2 (Utilities|Array|Add _outactors 0))
  (Utilities|FlowControl|Sequence
    (:then_0
      (Rendering|SetVisibility (Variables|Default|GetDefaultSceneRoot) (< _returnvalue_2 0) true)
      (Collision|SetActorEnableCollision (< _returnvalue_2 0))
      ;[0.8385 0.03057 0.03057 0.5] SE
      (if (< _returnvalue_2 0)
        (Utilities|FlowControl|DoOnce false
          (:Completed
            (Effects|SpawnEmitteratLocation "/Engine/Tutorial/SubEditors/TutorialAssets/TutorialParticleSystem.TutorialParticleSystem" _returnvalue)
            (Audio|PlaySoundatLocation "/Game/0_fps/Audio/MP3_Key_Appear.MP3_Key_Appear" _returnvalue "0, 0, 0" 1.0 1.0 0.0 0 0 0 0)))))
    (:then_1
      (Development|PrintString (Utilities|String|ToString(Integer) _returnvalue_2)))))

(fn ConstructionScript)